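; BPC_Timer is a stopwatch component that counts elapsed time and shows it through a WBP_Timer widget it creates at BeginPlay.
; Start resets the count, runs a looping timer that increments it and refreshes the widget, and plays the widget's ZoomOut animation.
; Pause, resume and stop act on the validated timer handle.
; Math-expression getters split the count into minutes, seconds and sub-second digits.
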(event Custom|Start_Timer
  (bind _timerwidget (Variables|Default|GetTimerWidget))
  (CallFunction|StopTimer)
  (Variables|Default|SetTime_millisec 0.0)
  (bind _returnvalue (Utilities|Time|SetTimerbyEvent (delegate Custom|Update%20Timer) (Variables|Default|GetIncrement) true))
  (Variables|Default|SetTimer%20Handle _returnvalue)
  (UserInterface|Animation|PlayAnimation _timerwidget (Variables|/Game/ProvidedAssets/Timer/WBP_Timer.WBP_Timer_C|GetZoomOut _timerwidget) 0.0 1 "Forward" 1.0 true))

(event Custom|Pause_Timer
  (bind _timer_handle (Utilities|ValidateHandle))
  (Utilities|Time|PauseTimerbyHandle _timer_handle))

(event Custom|Resume_Timer
  (bind _timer_handle (Utilities|ValidateHandle))
  (Utilities|Time|UnpauseTimerbyHandle _timer_handle))

(event Custom|Stop%20_Timer
  (bind _timer_handle (Utilities|ValidateHandle))
  (Utilities|Time|ClearandInvalidateTimerbyHandle _timer_handle))

(event Custom|Update%20Timer
  (Variables|Default|SetTime_millisec (+ (Variables|Default|GetTime_millisec) 1.0))
  (Default|Update (Variables|Default|GetTimerWidget)))

(event EventBeginPlay
  (bind _returnvalue (UserInterface|CreateWidget "/Game/ProvidedAssets/Timer/WBP_Timer.WBP_Timer_C" (Game|GetPlayerController 0)))
  (bind _output_get (Variables|Default|SetTimerWidget _returnvalue))
  (Variables|/Game/ProvidedAssets/Timer/WBP_Timer.WBP_Timer_C|SetTC _output_get self)
  (UserInterface|Viewport|AddtoViewport (Variables|Default|GetTimerWidget) 0))

(fn GetMS
  (return (|((floor((a/10)))%100) (Variables|Default|GetTime_millisec))))

(fn GetSec
  (return (|((floor((a/1000)))%60) (Variables|Default|GetTime_millisec))))

(fn GetMin
  (return (|(floor((((a/1000)/60)%60))) (Variables|Default|GetTime_millisec))))