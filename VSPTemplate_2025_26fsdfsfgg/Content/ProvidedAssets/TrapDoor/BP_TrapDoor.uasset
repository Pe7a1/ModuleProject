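; Trap door that closes when the player pawn leaves its trigger volume and reopens when the player re-enters it.
; End overlap plays a Timeline and begin overlap reverses it, lerping the door's relative location vertically with sweep enabled.
; The Construction Script derives the Timeline play rate from ClosingTimeInSec and offsets the trigger along local Y by TriggerDistance.
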(event `self.DoorTrigger.OnComponentBeginOverlap`
  (params (OverlappedComponent :type "PrimitiveComponent Object Reference") (OtherActor :type "Actor Object Reference") (OtherComp :type "PrimitiveComponent Object Reference") (OtherBodyIndex :type Integer) (bFromSweep :type Boolean) (SweepResult :type "HitResult Structure (by ref)"))
  (if (== OtherActor (`GameplayStatics.GetPlayerPawn` 0))
    (bind (_direction _output) (`Timeline|Timeline` :!via `Reverse` :!label _label)
      (:`Update`
        (`SceneComponent.K2_SetRelativeLocation` (`self.Door`) (`KismetMathLibrary.VLerp` (100.0 0.0 300.0) (100.0 0.0 0.0) _output) true false)))))

(event `self.DoorTrigger.OnComponentEndOverlap`
  (params (OverlappedComponent :type "PrimitiveComponent Object Reference") (OtherActor :type "Actor Object Reference") (OtherComp :type "PrimitiveComponent Object Reference") (OtherBodyIndex :type Integer))
  (if (== OtherActor (`GameplayStatics.GetPlayerPawn` 0))
    (goto _label)))

(fn `UserConstructionScript`
  (bind _doortrigger (`self.DoorTrigger`))
  (bind (_relativelocation_x _relativelocation_y _relativelocation_z) (`KismetMathLibrary.BreakVector` (`SceneComponent.RelativeLocation` _doortrigger)))
  (`TimelineComponent.SetPlayRate` (`self.Timeline`) (/ 1.0 (`self.ClosingTimeInSec`)))
  (`SceneComponent.K2_SetRelativeLocation` _doortrigger (`KismetMathLibrary.MakeVector` _relativelocation_x (`self.TriggerDistance`) _relativelocation_z) false false))